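; BP_Turret is an enemy turret that tracks and shoots at the player while they are inside its trigger box.
; A BP_Player entering the box starts two looping function-name timers instead of using Tick, and leaving clears both.
; FollowPlayer rotates the Pivot to look at player character 0, while FireAtPlayer spawns a BP_TurretProjectile at the ProjectileSpawn transform unless that spot is colliding.
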(event `FollowPlayer`
  (`SceneComponent.K2_SetWorldRotation` (`self.Pivot`) (`KismetMathLibrary.FindLookAtRotation` (`self.K2_GetActorLocation`) (`self.K2_GetActorLocation` (`GameplayStatics.GetPlayerCharacter` 0))) false false))

(event `FireAtPlayer`
  (`|SpawnActorFromClass` "/Game/Enemy/Turret/BP_TurretProjectile.BP_TurretProjectile_C" (`SceneComponent.K2_GetComponentToWorld` (`self.ProjectileSpawn`)) "DontSpawnIfColliding" "MultiplyWithRoot" null null))

(event `self.Box.OnComponentBeginOverlap`
  (params (OverlappedComponent :type "PrimitiveComponent Object Reference") (OtherActor :type "Actor Object Reference") (OtherComp :type "PrimitiveComponent Object Reference") (OtherBodyIndex :type Integer) (bFromSweep :type Boolean) (SweepResult :type "HitResult Structure (by ref)"))
  (cast `/Game/Player/BP_Player` OtherActor)
  (`KismetSystemLibrary.K2_SetTimer` null "FollowPlayer" 0.05 true)
  (`KismetSystemLibrary.K2_SetTimer` null "FireAtPlayer" 0.3 true))

(event `self.Box.OnComponentEndOverlap`
  (params (OverlappedComponent :type "PrimitiveComponent Object Reference") (OtherActor :type "Actor Object Reference") (OtherComp :type "PrimitiveComponent Object Reference") (OtherBodyIndex :type Integer))
  (cast `/Game/Player/BP_Player` OtherActor)
  (`KismetSystemLibrary.K2_ClearTimer` null "FollowPlayer")
  (`KismetSystemLibrary.K2_ClearTimer` null "FireAtPlayer"))

(fn `UserConstructionScript`)