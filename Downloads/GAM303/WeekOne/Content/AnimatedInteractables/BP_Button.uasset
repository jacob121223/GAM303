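; BP_Button is a color-coded pressure button that unlocks its target door when a physics pickup of the matching color overlaps it.
; The construction script tints the button through a dynamic material instance set to the pickup color.
; A match plays a timeline that lowers the button mesh.
; Any physics pickup ending overlap relocks the door and reverses the timeline, regardless of color.
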(event `self.Overlap.OnComponentBeginOverlap`
  (params (OverlappedComponent :type "PrimitiveComponent Object Reference") (OtherActor :type "Actor Object Reference") (OtherComp :type "PrimitiveComponent Object Reference") (OtherBodyIndex :type Integer) (bFromSweep :type Boolean) (SweepResult :type "HitResult Structure (by ref)"))
  (bind _asbp_physics_pickup (cast `/Game/Interactables/BP_PhysicsPickup` OtherActor))
  (if (== (`/Game/Interactables/BP_PhysicsPickup.PickupColor` _asbp_physics_pickup) (`self.Pickup Color`))
    (set `/Game/AnimatedInteractables/BP_Door.IsUnlocked` true (`self.TargetDoor`))
    (bind (_direction _alphatrack) (`Timeline|Alpha` :!label _label)
      (:`Update`
        (`SceneComponent.K2_SetRelativeLocation` (`self.Button`) (`KismetMathLibrary.MakeVector` 0.0 0.0 (`KismetMathLibrary.Lerp` 5.0 1.0 _alphatrack)) false false)))))

(event `self.Overlap.OnComponentEndOverlap`
  (params (OverlappedComponent :type "PrimitiveComponent Object Reference") (OtherActor :type "Actor Object Reference") (OtherComp :type "PrimitiveComponent Object Reference") (OtherBodyIndex :type Integer))
  (cast `/Game/Interactables/BP_PhysicsPickup` OtherActor)
  (set `/Game/AnimatedInteractables/BP_Door.IsUnlocked` false (`self.TargetDoor`))
  (goto _label :!via `Reverse`))

(fn `UserConstructionScript`
  (bind _returnvalue (`PrimitiveComponent.CreateDynamicMaterialInstance` (`self.Button`) 0 "/Game/Interactables/MAT_Color.MAT_Color" "None"))
  (bind _output_get (set `self.ColorDMI` _returnvalue))
  (`MaterialInstanceDynamic.SetVectorParameterValue` _output_get "Color" (`self.Pickup Color`)))